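; BP_ContenedorPieza is a base slot for object assembly that snaps a matching BP_Pieza to its hidden-by-default mesh transform.
; It caches overlapping slots as neighbours at BeginPlay and accepts pieces only once enabled.
; Placement triggers the overridable ObjetoColocado, which changes the piece's grab type and enables and reveals neighbours of the next type, filtered through RefObjeto.
; The completion check is hardcoded false, and end-overlap removal logic is disconnected.
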(event `self.ReceiveBeginPlay`
  (set `self.PoderColocarPieza` false)
  (`self.DesactivarMalla`)
  (for _array_element (`PrimitiveComponent.GetOverlappingActors` (`self.Collider`) "BP_ContenedorPieza_C")
    (`self.Filtrar/AgregarContenedores` _array_element)))

(event `self.Collider.OnComponentBeginOverlap`
  (params (OverlappedComponent :type "PrimitiveComponent Object Reference") (OtherActor :type "Actor Object Reference") (OtherComp :type "PrimitiveComponent Object Reference") (OtherBodyIndex :type Integer) (bFromSweep :type Boolean) (SweepResult :type "HitResult Structure (by ref)"))
  ;[0 0 0] Deteccion del objeto
  (`self.FiltrarColision` OtherActor
    (:`PiezaCorrecta`
      (if (`self.PoderColocarPieza`)
        (`self.DesactivarMalla`)
        (`self.ColocarPieza`)
        (`self.VerificarTerminacion`
          (:`ObjetoCompletado`
            ;;[0 0.3333 0.1038 1 14] Este método se sobrescribe en las clases heredadas.
            (`/Game/Proyecto/Blueprints/ArmarObjeto/BPI_ContenedorObjeto.ObjetoColocado`)
            (`/Game/Proyecto/Blueprints/ArmarObjeto/BPI_ContenedorObjeto.ObjetoCompletado`))
          (:`ObjetoIncompleto`
            (`/Game/Proyecto/Blueprints/ArmarObjeto/BPI_ContenedorObjeto.ObjetoColocado`)))))))

(event `/Game/Proyecto/Blueprints/ArmarObjeto/BPI_ContenedorObjeto.ObjetoColocado`
  ;[0 0 0] Deteccion del objeto
  (`self.CambiarGrabType` "NewEnumerator0")
  (`self.PoderColocarPiezaPorPieza` (`self.ContenedorSiguiente`) true)
  (`self.ActivarMallaPorPieza` (`self.ContenedorSiguiente`)))

(fn `ActivarMalla`
  (`SceneComponent.SetHiddenInGame` (`self.Malla`) false false))

(fn `ActivarMallaPorPieza`
  (params (TipoPieza :type "/Game/Proyecto/Blueprints/ArmarObjeto/Enum_PartesPieza Enum" :default "NewEnumerator0"))
  (locals (_GrabType :type "/Game/VRTemplate/Blueprints/GrabType Enum" :default "NewEnumerator0") (_ActivarMalla :type Boolean) (_ActivarCollider :type Boolean))
  (bind _listafiltrada (`self.FiltrarContenedoresPorPieza` TipoPieza)
    (:`SeFiltro`
      (for _array_element _listafiltrada
        (bind _contenedorsalida (`self.VerificarVecino` _array_element)
          (:`EsVecino`
            (`self.ActivarMalla` _contenedorsalida)))))))

(fn `ActivarVecinos`
  (if (!= 0 (`KismetArrayLibrary.Array_Length` (`self.RefContenedoresVecinos`)))
    (for _array_element (`self.RefContenedoresVecinos`)
      (`/Engine/EditorBlueprintResources/StandardMacros.IsValid` _array_element
        (:`Is Valid`
          (`self.ActivarMalla` _array_element))))))

(fn `CambiarGrabType`
  (params (GrabType :type "/Game/VRTemplate/Blueprints/GrabType Enum" :default "NewEnumerator0"))
  (bind _refpiezaactor (`self.RefPiezaActor`)
    (:`then`
      (`/Game/Proyecto/Blueprints/ArmarObjeto/BP_Pieza.CambiarGrabType` _refpiezaactor GrabType))
    (:`else`)))

(fn `CambiarGrabTypeDeContenedoresPorPieza`
  (params (TipoPieza :type "/Game/Proyecto/Blueprints/ArmarObjeto/Enum_PartesPieza Enum" :default "NewEnumerator0") (GrabType :type "/Game/VRTemplate/Blueprints/GrabType Enum" :default "NewEnumerator0"))
  (bind _listafiltrada (`self.FiltrarContenedoresPorPieza` TipoPieza)
    (:`SeFiltro`
      (for _array_element _listafiltrada
        (`/Engine/EditorBlueprintResources/StandardMacros.IsValid` _array_element
          (:`Is Valid`
            (`self.CambiarGrabType` _array_element GrabType)))))))

(fn `ColocarPieza`
  (bind _malla (`self.Malla`))
  (`/Game/Proyecto/Blueprints/ArmarObjeto/BP_Pieza.EnColocar` (`self.RefPiezaActor`) (`SceneComponent.K2_GetComponentLocation` _malla) (`SceneComponent.K2_GetComponentRotation` _malla))
  (message `/Game/Proyecto/Blueprints/ArmarObjeto/BPI_Pieza.ColocarPieza` (`self.RefPiezaActor`)))

(fn `Desactivar Vecinos`
  (if (!= 0 (`KismetArrayLibrary.Array_Length` (`self.RefContenedoresVecinos`)))
    (for _array_element (`self.RefContenedoresVecinos`)
      (`/Engine/EditorBlueprintResources/StandardMacros.IsValid` _array_element
        (:`Is Valid`
          (`self.DesactivarMalla` _array_element))))))

(fn `DesactivarMalla`
  (`SceneComponent.SetHiddenInGame` (`self.Malla`) true false))

(fn `DesactivarMallaPorPieza`
  (params (TipoPieza :type "/Game/Proyecto/Blueprints/ArmarObjeto/Enum_PartesPieza Enum" :default "NewEnumerator0"))
  (locals (_GrabType :type "/Game/VRTemplate/Blueprints/GrabType Enum" :default "NewEnumerator0") (_ActivarMalla :type Boolean) (_ActivarCollider :type Boolean))
  (bind _listafiltrada (`self.FiltrarContenedoresPorPieza` TipoPieza)
    (:`SeFiltro`
      (for _array_element _listafiltrada
        (bind _contenedorsalida (`self.VerificarVecino` _array_element)
          (:`EsVecino`
            (`self.DesactivarMalla` _contenedorsalida)))))))

(fn `EscupirPiezaDeContendoresVecinos`
  (params (PartePieza :type "/Game/Proyecto/Blueprints/ArmarObjeto/Enum_PartesPieza Enum" :default "NewEnumerator0"))
  (bind _listafiltrada (`self.FiltrarContenedoresPorPieza` PartePieza)
    (:`SeFiltro`
      (for _array_element _listafiltrada
        (bind _contenedorsalida (`self.VerificarVecino` _array_element)
          (:`EsVecino`
            (bind _contendorsalida (`self.VerificarContenedorOcupado` _contenedorsalida)
              (:`Ocupado`
                (bind _refpiezaactor (`/Game/Proyecto/Blueprints/ArmarObjeto/BP_ContenedorPieza.RefPiezaActor` _contendorsalida)
                  (:`then`
                    (`/Game/Proyecto/Blueprints/ArmarObjeto/BP_Pieza.AsignarSimulacionFisicas` _refpiezaactor true)
                    (set `/Game/VRTemplate/Blueprints/GrabComponent.GrabType` "NewEnumerator4" (`/Game/Proyecto/Blueprints/ArmarObjeto/BP_Pieza.GrabComponent` _refpiezaactor)))
                  (:`else`))))))))))

(fn `PoderColocarPiezaPorPieza`
  (params (TipoPieza :type "/Game/Proyecto/Blueprints/ArmarObjeto/Enum_PartesPieza Enum" :default "NewEnumerator0") (_PoderColocarPieza :type Boolean))
  (locals (_GrabType :type "/Game/VRTemplate/Blueprints/GrabType Enum" :default "NewEnumerator0") (_ActivarMalla :type Boolean) (_ActivarCollider :type Boolean))
  (bind _listafiltrada (`self.FiltrarContenedoresPorPieza` TipoPieza)
    (:`SeFiltro`
      (for _array_element _listafiltrada
        (bind _contenedorsalida (`self.VerificarVecino` _array_element)
          (:`EsVecino`
            (set `/Game/Proyecto/Blueprints/ArmarObjeto/BP_ContenedorPieza.PoderColocarPieza` _PoderColocarPieza _contenedorsalida)))))))

(fn `UserConstructionScript`)

(fn `VerificarContendoresOcupadosPorTipo`
  (params (TipoPieza :type "/Game/Proyecto/Blueprints/ArmarObjeto/Enum_PartesPieza Enum" :default "NewEnumerator0"))
  (returns (Ocupados :type Boolean))
  (locals (ContendoresOcupado :type Boolean))
  (bind _listafiltrada (`self.FiltrarContenedoresPorPieza` TipoPieza)
    (:`SeFiltro`
      (set `local.ContendoresOcupado` false)
      (for _array_element _listafiltrada
        (bind _contenedorsalida (`self.VerificarVecino` _array_element)
          (:`EsVecino`
            (if (`/Game/Proyecto/Blueprints/ArmarObjeto/BP_ContenedorPieza.bPiezaOcupada` _contenedorsalida)
              (set `local.ContendoresOcupado` true)))))
      (return (`local.ContendoresOcupado`)))))