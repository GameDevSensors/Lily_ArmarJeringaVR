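; BP_Pieza_3_A is a grabbable syringe (Jeringa) piece that detaches when picked up and unlocks the next cap.
; On grab it force-releases through its GrabComponent; on success it changes its grab type, detaches keeping world transform, makes TapaB grabbable and disables its own grabbing.
; On drop it enables physics on the Pieza component.
; Unwired leftover nodes for physics, TapaB grab type and delayed destruction never run.
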(event `self.ReceiveBeginPlay`
  (`parent.ReceiveBeginPlay`))

(event `self.GrabComponent.OnGrabbed`
  (bind _grabcomponent (`self.GrabComponent`))
  ;[0 0 0] Soltar pieza
  (bind _breleased (`/Game/VRTemplate/Blueprints/GrabComponent.TryRelease` _grabcomponent))
  (if _breleased
    (set `/Game/VRTemplate/Blueprints/GrabComponent.GrabType` "NewEnumerator0" _grabcomponent)
    (`self.K2_DetachFromActor` "KeepWorld" "KeepWorld" "KeepWorld")
    (`self.Agarrable` (`self.Tapa_B`))
    (`self.NoAgarrable`)))

(event `self.GrabComponent.OnDropped`
  (`PrimitiveComponent.SetSimulatePhysics` (`self.Pieza`) true))

(fn `UserConstructionScript`
  (`parent.UserConstructionScript`))