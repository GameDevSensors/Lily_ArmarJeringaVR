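; BP_Pieza_1_Base is the base piece of a syringe (Jeringa) assembly that receives the BP_Tapa_B cap.
; When the cap overlaps its Box, it attaches the cap to itself, moves it to the Box's relative location and calls DesbloquearTapa on it.
; Older logic for filtering and attaching BP_Pieza_3_C and setting the grab type remains in the graph but is unconnected.
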(event `self.Box.OnComponentBeginOverlap`
  (params (OverlappedComponent :type "PrimitiveComponent Object Reference") (OtherActor :type "Actor Object Reference") (OtherComp :type "PrimitiveComponent Object Reference") (OtherBodyIndex :type Integer) (bFromSweep :type Boolean) (SweepResult :type "HitResult Structure (by ref)"))
  (bind _asbp_tapa_b (cast `/Game/Proyecto/Blueprints/Jeringa/BP_Tapa_B` OtherActor))
  (`self.K2_AttachToActor` _asbp_tapa_b self "None" "SnapToTarget" "SnapToTarget" "SnapToTarget" true)
  (`self.K2_SetActorRelativeLocation` _asbp_tapa_b (`SceneComponent.RelativeLocation` (`self.Box`)) false false)
  (`/Game/Proyecto/Blueprints/Jeringa/BP_Tapa_B.DesbloquearTapa` _asbp_tapa_b))

(fn `UserConstructionScript`
  (`parent.UserConstructionScript`))