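; BP_Pieza_Jeringa is a syringe piece Blueprint with helpers for joining it to other pieces.
; FiltrarPieza casts an actor to BP_Pieza, stores it in RefPiezaJuntar, and checks that its piece type and GrabComponent grab type match the required values.
; AtacharPieza snaps a given piece onto this actor, then positions it at the relative location of a supplied scene component.
; The event graph holds no active logic.
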(fn `AtacharPieza`
  (params (PiezaAtachar :type "Actor Object Reference") (SceneComponentAtachar :type "SceneComponent Object Reference"))
  (`self.K2_AttachToActor` PiezaAtachar self "None" "SnapToTarget" "SnapToTarget" "SnapToTarget" true)
  (`self.K2_SetActorRelativeLocation` PiezaAtachar (`SceneComponent.RelativeLocation` SceneComponentAtachar) false false))

(fn `FiltrarPieza`
  (params (Actor :type "Actor Object Reference") (PartesPieza :type "/Game/Proyecto/Blueprints/ArmarObjeto/Enum_PartesPieza Enum" :default "NewEnumerator14"))
  (returns (EsPieza :type Boolean))
  (bind _asbp_pieza (cast `/Game/Proyecto/Blueprints/ArmarObjeto/BP_Pieza` Actor)
    (:`then`
      (bind _output_get (set `self.RefPiezaJuntar` _asbp_pieza))
      (return (and (`|EnumEquality` (`/Game/Proyecto/Blueprints/ArmarObjeto/BP_Pieza.TipoPieza` _output_get) PartesPieza) (`|EnumEquality` "NewEnumerator4" (`/Game/VRTemplate/Blueprints/GrabComponent.GrabType` (`self.GetComponentByClass` _asbp_pieza "/Game/VRTemplate/Blueprints/GrabComponent.GrabComponent_C"))))))
    (:`CastFailed`
      (return false))))

(fn `UserConstructionScript`
  (`parent.UserConstructionScript`))