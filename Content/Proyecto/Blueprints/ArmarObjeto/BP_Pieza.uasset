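; BP_Pieza is a grabbable VR piece for object assembly that can be placed at a given position and rotation.
; On EnColocar it releases itself from the VRPawn hand holding it, snaps to that transform and turns off physics on its root mesh.
; Helper functions switch the GrabComponent's grab type to make the piece grabbable or not, while their collision and tick changes are left disconnected.
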(event `self.ReceiveBeginPlay`
  (bind _asvrpawn (cast `/Game/VRTemplate/Blueprints/VRPawn` (`GameplayStatics.GetPlayerPawn` 0)))
  (set `self.RefVRPawn` _asvrpawn))

(event `EnColocar`
  (params (Posicion :type "Vector Structure") (Rotacion :type "Rotator Structure"))
  (`self.LiberarMano`)
  ;[0 0 0] Asignacion de configuraciones al objeto agarrado
  (`self.AsignarPosicion` Posicion)
  (`self.AsignarRotacion` Rotacion)
  (`self.AsignarSimulacionFisicas` false))

(fn `Agarrable`
  (set `/Game/VRTemplate/Blueprints/GrabComponent.GrabType` "NewEnumerator1" (`self.GrabComponent`)))

(fn `AsignarPosicion`
  (params (NuevaPosicion :type "Vector Structure"))
  (`self.K2_SetActorLocation` NuevaPosicion))

(fn `AsignarRotacion`
  (params (NuevaRotacion :type "Rotator Structure"))
  (`self.K2_SetActorRotation` NuevaRotacion))

(fn `AsignarSimulacionFisicas`
  (params (Simulacion :type Boolean))
  (bind _asmesh_component (cast `MeshComponent` (`self.RootComponent`)))
  (`PrimitiveComponent.SetSimulatePhysics` _asmesh_component Simulacion))

(fn `CambiarGrabType`
  (params (GrabType :type "/Game/VRTemplate/Blueprints/GrabType Enum" :default "NewEnumerator0"))
  (set `/Game/VRTemplate/Blueprints/GrabComponent.GrabType` GrabType (`self.GrabComponent`)))

(fn `LiberarMano`
  (if (`|EnumEquality` "Right" (`/Game/VRTemplate/Blueprints/GrabComponent.GetHeldByHand` (`self.GrabComponent`)))
    (bind _heldcomponentright (`/Game/VRTemplate/Blueprints/VRPawn.HeldComponentRight` (`self.RefVRPawn`))
      (:`then`
        (bind _breleased (`/Game/VRTemplate/Blueprints/GrabComponent.TryRelease` _heldcomponentright))
        (if _breleased
          (set `/Game/VRTemplate/Blueprints/VRPawn.HeldComponentRight` null (`self.RefVRPawn`))))
      (:`else`))
    (else
      (bind _heldcomponentleft (`/Game/VRTemplate/Blueprints/VRPawn.HeldComponentLeft` (`self.RefVRPawn`))
        (:`then`
          (bind _breleased_2 (`/Game/VRTemplate/Blueprints/GrabComponent.TryRelease` _heldcomponentleft))
          (if _breleased_2
            (set `/Game/VRTemplate/Blueprints/VRPawn.HeldComponentLeft` null (`self.RefVRPawn`))))
        (:`else`)))))

(fn `NoAgarrable`
  (set `/Game/VRTemplate/Blueprints/GrabComponent.GrabType` "NewEnumerator0" (`self.GrabComponent`)))

(fn `UserConstructionScript`)