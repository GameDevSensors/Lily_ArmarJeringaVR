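; BP_Objeto is an object in the object-assembly system (ArmarObjeto) that manages the containers where its pieces go.
; On BeginPlay it gathers its BP_ContenedorPieza child actors into an array and gives each a back-reference to itself.
; FiltrarContenedoresPorPieza uses the FiltroContenedores macro to return the valid, unique containers that accept a given piece type, with their count and a success flag.
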(event `self.ReceiveBeginPlay`
  (`self.ReferenciarContenedores`))

(fn `FiltrarContenedoresPorPieza`
  (params (TipoPieza :type "/Game/Proyecto/Blueprints/ArmarObjeto/Enum_PartesPieza Enum" :default "NewEnumerator0"))
  (returns (`SeFiltro?` :type Boolean) (ElementosFIltrados :type "Array of /Game/Proyecto/Blueprints/ArmarObjeto/BP_ContenedorPieza Object Reference") (CantidadElementosFiltrados :type Integer))
  (locals (SeFiltro :type Boolean))
  (bind _cantidadelementosfiltrados (`self.FiltroContenedores` TipoPieza)
    (:`SeFiltranElementos`
      (bind _output_get (set `local.SeFiltro` true))
      (return _output_get (`self.ContenedoresFiltrados`) _cantidadelementosfiltrados))
    (:`NoSeFiltranElementos`
      (bind _output_get_2 (set `local.SeFiltro` false))
      (return _output_get_2 _ 0))))

(fn `ReferenciarContenedores`
  (for _array_element (`self.GetAllChildActors` false)
    (bind _asbp_contenedor_pieza (cast `/Game/Proyecto/Blueprints/ArmarObjeto/BP_ContenedorPieza` _array_element))
    (set `/Game/Proyecto/Blueprints/ArmarObjeto/BP_ContenedorPieza.RefObjeto` self _asbp_contenedor_pieza)
    (`KismetArrayLibrary.Array_Add` (`self.RefContenedoresPieza`) _asbp_contenedor_pieza)))

(fn `UserConstructionScript`)