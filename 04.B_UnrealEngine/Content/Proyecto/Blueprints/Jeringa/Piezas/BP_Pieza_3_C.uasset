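; BP_Pieza_3_C is a syringe piece (Jeringa) that lets its first cap be removed once it touches the piece's base.
; On Box overlap, FiltrarPieza casts the other actor to BP_Pieza, stores the reference and compares its TipoPieza to the expected type.
; A match makes TapaA grabbable, then disables collision and component tick on the Pieza component.
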(event `self.ReceiveBeginPlay`
  (`parent.ReceiveBeginPlay`))

(event `self.Box.OnComponentBeginOverlap`
  (params (OverlappedComponent :type "PrimitiveComponent Object Reference") (OtherActor :type "Actor Object Reference") (OtherComp :type "PrimitiveComponent Object Reference") (OtherBodyIndex :type Integer) (bFromSweep :type Boolean) (SweepResult :type "HitResult Structure (by ref)"))
  (bind _pieza (`self.Pieza`))
  ;[0 0 0] Verifica que se colisiona con la base de la pieza para poder sacar la primer tapa
  (bind _espieza (`self.FiltrarPieza` OtherActor "NewEnumerator8"))
  (if _espieza
    (`self.Agarrable` (`self.Tapa_A`))
    (`PrimitiveComponent.SetCollisionEnabled` _pieza "NoCollision")
    (`ActorComponent.SetComponentTickEnabled` _pieza false)))

(fn `FiltrarPieza`
  (params (Actor :type "Actor Object Reference") (PartesPieza :type "/Game/Proyecto/Blueprints/ArmarObjeto/Enum_PartesPieza Enum" :default "NewEnumerator14"))
  (returns (EsPieza :type Boolean))
  (bind _asbp_pieza (cast `/Game/Proyecto/Blueprints/ArmarObjeto/BP_Pieza` Actor)
    (:`then`
      (bind _output_get (set `self.RefPiezaJuntar` _asbp_pieza))
      (return (`|EnumEquality` (`/Game/Proyecto/Blueprints/ArmarObjeto/BP_Pieza.TipoPieza` _output_get) PartesPieza)))
    (:`CastFailed`
      (return false))))

(fn `UserConstructionScript`
  (`parent.UserConstructionScript`))